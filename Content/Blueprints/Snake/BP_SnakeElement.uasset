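; BP_SnakeElement is a single segment of a snake, providing the visuals for its head, body and tail pieces.
; Separate events swap the mesh component between head, body and tail static meshes, and the head event also rescales the actor.
; A material event uses a FlipFlop to alternate between an opacity material and the normal snake material on each call.
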(event EventSetLastElementMesh
  (Components|StaticMesh|SetStaticMesh (Variables|Default|GetmeshComponent) "/Game/Blueprints/Assets/SnakeElement/TailSnake.TailSnake"))

(event EventSetFirstElementMesh
  (Components|StaticMesh|SetStaticMesh (Variables|Default|GetmeshComponent) "/Game/Blueprints/Assets/SnakeHead/SnakeHead.SnakeHead")
  (Transformation|SetActorScale3D "0.380000,0.380000,0.380000"))

(event EventSetElementsMesh
  (Components|StaticMesh|SetStaticMesh (Variables|Default|GetmeshComponent) "/Game/Blueprints/Assets/SnakeElement/SnakeElement.SnakeElement"))

(event EventSetSnakeMaterial
  (Utilities|FlowControl|FlipFlop
    (:A
      (Rendering|Material|SetMaterial (Variables|Default|GetmeshComponent) 0 "/Game/Blueprints/Assets/SnakeHead/M_SnakeOpacityMaterial.M_SnakeOpacityMaterial"))
    (:B
      (Rendering|Material|SetMaterial (Variables|Default|GetmeshComponent) 0 "/Game/Blueprints/Assets/SnakeHead/SnakeMaterial.SnakeMaterial"))))

(fn ConstructionScript)